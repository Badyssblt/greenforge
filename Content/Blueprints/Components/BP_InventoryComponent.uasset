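; Inventory component that stores items in a map of numbered slots, each holding an item ID and a count.
; BeginPlay fills MaxSlot slots with an empty-item enum value, then adds two hardcoded stacks of the same item.
; AddItem writes to the first slot that is empty or holds the same ID, summing counts on a match, with no stack limit.
; RefreshItem, HasItem and EnoughSpace are empty stubs.
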(event `self.ReceiveBeginPlay`
  (`self.InitInventory`)
  (`self.AddItem` (make `/Game/Data/Structs/S_ItemCount` "NewEnumerator0" 3))
  (`self.AddItem` (make `/Game/Data/Structs/S_ItemCount` "NewEnumerator0" 2)))

(fn `AddItem`
  (params (toAdd :type "/Game/Data/Structs/S_ItemCount Structure"))
  (locals (CurrentSlot :type Integer) (CountToAdd :type Integer))
  (bind _toadd_itemid (break `/Game/Data/Structs/S_ItemCount` (`local.toAdd`)))
  (bind (_toadd_itemid_2 _toadd_count) (break `/Game/Data/Structs/S_ItemCount` (`local.toAdd`)))
  (bind _toadd_itemid_3 (break `/Game/Data/Structs/S_ItemCount` (`local.toAdd`)))
  (bind _value (`BlueprintMapLibrary.Map_Find` (`self.Items`) (`local.CurrentSlot`)))
  (bind _keys (`BlueprintMapLibrary.Map_Keys` (`self.Items`)))
  (for _array_element _keys
    (set `local.CurrentSlot` _array_element)
    (if (`|EnumEquality` (break `/Game/Data/Structs/S_ItemCount` (`BlueprintMapLibrary.Map_Find` (`self.Items`) (`local.CurrentSlot`))) "NewEnumerator1")
      ; Ajoute l'item à l'inventory
      (`BlueprintMapLibrary.Map_Remove` (`self.Items`) (`local.CurrentSlot`))
      (`BlueprintMapLibrary.Map_Add` (`self.Items`) (`local.CurrentSlot`) (`local.toAdd`))
      (break)
      (else
        ; Ajoute le count du toAdd à l'item déjà présent dans l'inventory
        (if (`|EnumEquality` (break `/Game/Data/Structs/S_ItemCount` _value) _toadd_itemid)
          (set `local.CountToAdd` (+ (`.Count_5_DA90FAE54F0983B547C67BA1EAD803C0` (break `/Game/Data/Structs/S_ItemCount` _value)) _toadd_count))
          (`BlueprintMapLibrary.Map_Remove` (`self.Items`) (`local.CurrentSlot`))
          (`BlueprintMapLibrary.Map_Add` (`self.Items`) (`local.CurrentSlot`) (make `/Game/Data/Structs/S_ItemCount` _toadd_itemid_3 (`local.CountToAdd`)))
          (break))))))

(fn `EnoughSpace`)

(fn `HasItem`)

(fn `InitInventory`
  (locals (SlotID :type Integer))
  (for _index (range 1 (+ (`self.MaxSlot`) 1))
    (bind _output_get (set `local.SlotID` _index))
    (`BlueprintMapLibrary.Map_Add` (`self.Items`) _output_get (make `/Game/Data/Structs/S_ItemCount` "NewEnumerator1"))))

(fn `RefreshItem`)