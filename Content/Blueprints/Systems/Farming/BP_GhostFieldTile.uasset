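; BP_GhostFieldTile is an interactable farming tile that plants and harvests a crop.
; Interact harvests CurrentCrop when ready; otherwise it attempts planting, even if an unripe crop already occupies the tile.
; Planting takes the crop data's seed from the inventory, spawns a BP_CropPlant linked to the tile and starts growth, or prints a no-seed message.
; Harvesting adds the crop's item to the inventory and destroys the plant.
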(event `self.Interact`
  (bind _currentcrop (`self.CurrentCrop`))
  (`/Engine/EditorBlueprintResources/StandardMacros.IsValid` _currentcrop
    (:`Is Valid`
      (if (`/Game/Blueprints/Systems/Farming/BP_CropPlant.CanHarvest` _currentcrop)
        (`self.HarvestCrop`)
        (else
          (`self.PlantCrop` :!label _label))))
    (:`Is Not Valid`
      (goto _label))))

(fn `HarvestCrop`
  (bind (_cropdata_name _cropdata_growthstage _cropdata_timetogrow _cropdata_mesh _cropdata_item) (break `/Game/Data/Structs/Farming/S_CropData` (`/Game/Blueprints/Library/BFL_Crop.GetCropData` (`/Game/Blueprints/Systems/Farming/BP_CropPlant.Plant` (`self.CurrentCrop`)))))
  (`/Game/Blueprints/Components/BP_InventoryComponent.AddItem` (`/Game/Blueprints/Library/BFL_Inventory.GetInventory`) _cropdata_item)
  (`self.K2_DestroyActor` (`self.CurrentCrop`)))

(fn `PlantCrop`
  (bind (_cropdata_name _cropdata_growthstage _cropdata_timetogrow _cropdata_mesh _cropdata_item _cropdata_mincount _cropdata_maxcount _cropdata_replantable _cropdata_seed) (break `/Game/Data/Structs/Farming/S_CropData` (`/Game/Blueprints/Library/BFL_Crop.GetCropData` (`self.Plant`))))
  (bind _item_itemid (break `/Game/Data/Structs/Items/S_ItemCount` (`/Game/Blueprints/Components/BP_InventoryComponent.HasItem` (`/Game/Blueprints/Library/BFL_Inventory.GetInventory`) _cropdata_seed)))
  (if (`|EnumInequality` _item_itemid "NewEnumerator1")
    (`/Game/Blueprints/Components/BP_InventoryComponent.RemoveItem` (`/Game/Blueprints/Library/BFL_Inventory.GetInventory`) _cropdata_seed)
    (bind _returnvalue (`|SpawnActorFromClass` "/Game/Blueprints/Systems/Farming/BP_CropPlant.BP_CropPlant_C" (`self.GetTransform`) "Undefined" "MultiplyWithRoot" null (`self.Plant`) self null))
    (bind _output_get (set `self.CurrentCrop` _returnvalue))
    (`/Game/Blueprints/Systems/Farming/BP_CropPlant.StartGrowth` _returnvalue)
    (`/Game/Blueprints/Systems/Farming/BP_CropPlant.StartGrowth` _output_get)
    (else
      (`KismetSystemLibrary.PrintString` "Pas de seed !"))))

(fn `UserConstructionScript`)