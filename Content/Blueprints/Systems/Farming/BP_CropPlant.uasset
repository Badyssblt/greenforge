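; BP_CropPlant is a farming crop plant that grows through timed stages until it is ready to harvest.
; StartGrowth calls AdvanceGrowth, which reads the stage count and time per stage from GetCropData for its Plant.
; AdvanceGrowth re-calls itself after each Delay, incrementing CurrentStage and setting the Stage enum, then marks the crop harvestable, with French debug prints.
; Its OR-ed not-equal guard on Stage always passes, so only the stage count ends growth.
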(event `AdvanceGrowth`
  (bind _stage (`self.Stage`))
  (bind (_cropdata_name _cropdata_growthstage _cropdata_timeperstage) (break `/Game/Data/Structs/Farming/S_CropData` (`/Game/Blueprints/Library/BFL_Crop.GetCropData` (`self.Plant`))))
  (if (or (`|EnumInequality` _stage "NewEnumerator2") (`|EnumInequality` _stage "NewEnumerator3"))
    (if (<= (`self.CurrentStage`) _cropdata_growthstage)
      (`KismetSystemLibrary.Delay` _cropdata_timeperstage)
      (`/Engine/EditorBlueprintResources/StandardMacros.IncrementInt` (`self.CurrentStage`)
        (:`  `
          (set `self.Stage` "NewEnumerator1")
          (`KismetSystemLibrary.PrintString` "En train de pousser")
          (`self.AdvanceGrowth`)))
      (else
        (set `self.Stage` "NewEnumerator2")
        (`KismetSystemLibrary.PrintString` "La plante est prête à être récolté!")))))

(fn `StartGrowth`
  (`self.AdvanceGrowth`))

(fn `UserConstructionScript`)