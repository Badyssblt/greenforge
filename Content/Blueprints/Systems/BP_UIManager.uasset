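; BP_UIManager creates the inventory UI and fills it with item slots.
; InitWidgets creates WBP_Inventory, stores the reference and adds it to the viewport.
; RefreshInventory clears the widget's uniform grid, then creates a WBP_Slot for each key in the inventory's Items map, passing its slot ID and item.
; Row and Column counters lay the slots out five per row.
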(fn `InitWidgets`
  (bind _returnvalue (`|CreateWidget` "/Game/Blueprints/UI/Inventory/WBP_Inventory.WBP_Inventory_C"))
  (bind _output_get (set `self.InventoryWidget` _returnvalue))
  (`UserWidget.AddToViewport` _output_get 0))

(fn `RefreshInventory`
  (locals (SlotID :type Integer) (ItemSlot :type "/Game/Data/Structs/S_ItemCount Structure") (SlotRef :type "/Game/Blueprints/UI/Inventory/WBP_Slot Object Reference") (Row :type Integer) (Column :type Integer))
  (`PanelWidget.ClearChildren` (`/Game/Blueprints/UI/Inventory/WBP_Inventory.UGP_Items` (`self.InventoryWidget`)))
  (bind _keys (`BlueprintMapLibrary.Map_Keys` (`/Game/Blueprints/Components/BP_InventoryComponent.Items` (`/Game/Blueprints/Library/BFL_Inventory.GetInventory`))))
  (for _array_element _keys
    (if (>= (`local.Column`) 5)
      (set `local.Column` 0)
      (`/Engine/EditorBlueprintResources/StandardMacros.IncrementInt` (`local.Row`)
        (:`  `
          _)))
    (set `local.SlotID` _array_element)
    (set `local.ItemSlot` (`BlueprintMapLibrary.Map_Find` (`/Game/Blueprints/Components/BP_InventoryComponent.Items` (`/Game/Blueprints/Library/BFL_Inventory.GetInventory`)) (`local.SlotID`)))
    (bind _returnvalue (`|CreateWidget` "/Game/Blueprints/UI/Inventory/WBP_Slot.WBP_Slot_C" null (`local.SlotID`) (`local.ItemSlot`)))
    (bind _output_get (set `local.SlotRef` _returnvalue))
    (`UniformGridPanel.AddChildToUniformGrid` (`/Game/Blueprints/UI/Inventory/WBP_Inventory.UGP_Items` (`self.InventoryWidget`)) _output_get (`local.Row`) (`local.Column`))
    (`/Engine/EditorBlueprintResources/StandardMacros.IncrementInt` (`local.Column`))))